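; MyGhostBP is a ghost pawn that can steal control of a MyCharacterBP the player looks at, apparently as a test feature.
; Pressing Tab fires a debug-drawn Visibility line trace forward from the follow camera.
; If it hits a MyCharacterBP, the two controllers swap pawns: the ghost's controller possesses the character and the character's controller possesses the ghost.
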(event `Key|Tab`
  (params (Key :type "Key Structure"))
  (:`Pressed`
    (`self.TestStealFunc`)))

(event `TestStealFunc`
  (bind _followcamera (`self.FollowCamera`))
  (bind _returnvalue (`SceneComponent.K2_GetComponentLocation` _followcamera))
  (bind _outhit (`KismetSystemLibrary.LineTraceSingle` :`Start` _returnvalue :`End` (+ _returnvalue (* (`SceneComponent.GetForwardVector` _followcamera) 1000.0)) :`TraceChannel` "TraceTypeQuery1" :`DrawDebugType` "ForDuration"))
  (bind _asmy_character_bp (cast `/Game/Blueprints/MyCharacterBP` (`.HitActor` (`GameplayStatics.BreakHitResult` _outhit))))
  (set `self.GhostControllerBP` (`self.GetController`))
  (set `self.CharacterControllerBP` (`self.GetController` _asmy_character_bp))
  (`Controller.Possess` (`self.GhostControllerBP`) _asmy_character_bp)
  (`Controller.Possess` (`self.CharacterControllerBP`) self))

(event `self.ReceiveBeginPlay`)

(fn `UserConstructionScript`)